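; Player controller for mouse-driven movement and building, with a visible cursor, a build widget toggled by F and a money readout set once at BeginPlay.
; Left click traces under the cursor and sends the hit point to the AI controller of the player's MyCharacter.
; Right click traces likewise, then box-traces above the hit to spawn BP_MyBuild if clear or print a warning if blocked, independent of build widget visibility.
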(event `self.ReceiveBeginPlay`
  (set `self.bShowMouseCursor` true)
  (bind _returnvalue (`|CreateWidget` "/Game/BP_MyWidget.BP_MyWidget_C"))
  (bind _output_get (set `self.UI_Build` _returnvalue))
  (`UserWidget.AddToViewport` _output_get 1)
  (`Widget.SetVisibility` (`self.UI_Build`) "Hidden")
  (bind _returnvalue_2 (`|CreateWidget` "/Game/BP_WidgetMoney.BP_WidgetMoney_C"))
  (bind _output_get_2 (set `self.UI_Money` _returnvalue_2))
  (`UserWidget.AddToViewport` _output_get_2 0)
  (`Widget.SetVisibility` (`self.UI_Money`) "Visible")
  (bind _asbp_my_player (cast `/Game/BP_MyPlayer` (`GameplayStatics.GetPlayerCharacter` 0)))
  (`TextBlock.SetText` (`/Game/BP_WidgetMoney.Money` (`self.UI_Money`)) (`KismetTextLibrary.Conv_StringToText` (`KismetStringLibrary.Concat_StrStr` "Money: " (`KismetStringLibrary.Conv_IntToString` (`/Game/BP_MyPlayer.Money` _asbp_my_player))))))

(event `Key|LeftMouseButton`
  (params (Key :type "Key Structure"))
  (bind (_worldlocation _worlddirection) (`self.DeprojectMousePositionToWorld`))
  ;[1 1 1] Where to go
  (:`Pressed`
    (bind _asbp_my_player (cast `/Game/BP_MyPlayer` (`GameplayStatics.GetPlayerCharacter` 0)))
    (bind _asbp_my_aicontroller (cast `/Game/BP_MyAIController` (`Pawn.GetController` (`/Game/BP_MyPlayer.MyCharacter` _asbp_my_player))))
    (bind (_outhit _returnvalue) (`KismetSystemLibrary.LineTraceSingle` _worldlocation (+ _worldlocation (* _worlddirection 2000.0)) "TraceTypeQuery1"))
    (if _returnvalue
      (`/Game/BP_MyAIController.GoToLocationMouse` _asbp_my_aicontroller (`.Location` (`GameplayStatics.BreakHitResult` _outhit))))))

(event `Key|F`
  (params (Key :type "Key Structure"))
  (bind _ui_build (`self.UI_Build`))
  (:`Pressed`
    (bind _output_get (set `self.isShowUI` (not (`self.isShowUI`))))
    (if _output_get
      (`Widget.SetVisibility` _ui_build "Visible")
      (else
        (`Widget.SetVisibility` _ui_build "Hidden")))))

(event `Key|RightMouseButton`
  (params (Key :type "Key Structure"))
  (bind (_worldlocation _worlddirection) (`self.DeprojectMousePositionToWorld`))
  (:`Pressed`
    (bind (_outhit _returnvalue) (`KismetSystemLibrary.LineTraceSingle` _worldlocation (+ _worldlocation (* _worlddirection 2000.0)) "TraceTypeQuery1"))
    (if _returnvalue
      (bind _returnvalue_2 (+ (`.Location` (`GameplayStatics.BreakHitResult` _outhit)) (0.0 0.0 85.0)))
      (bind (_outhit_2 _returnvalue_3) (`KismetSystemLibrary.BoxTraceSingle` :`Start` _returnvalue_2 :`End` _returnvalue_2 :`HalfSize` (100.0 100.0 80.0) :`TraceChannel` "TraceTypeQuery1" :`DrawTime` 3.0))
      (if _returnvalue_3
        (`KismetSystemLibrary.PrintString` "You can't build here!")
        (else
          (`|SpawnActorFromClass` "/Game/BP_MyBuild.BP_MyBuild_C" (`KismetMathLibrary.MakeTransform` (`.Location` (`GameplayStatics.BreakHitResult` _outhit))) "DontSpawnIfColliding" "OverrideRootScale" null null))))))

(fn `UserConstructionScript`)